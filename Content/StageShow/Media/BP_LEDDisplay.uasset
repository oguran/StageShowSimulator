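; BP_LEDDisplay is a stage-show LED display actor whose event graph serves as a keyboard debug harness for its LedMediaPlayback member.
; Number keys call open, play, pause, stop and seek, printing whether each request succeeded.
; Seek tests include negative and far out-of-range times.
; Further keys print duration, current media time and the open-pending and opened states.
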(event `Key|One`
  (params (Key :type "Key Structure"))
  (:`Pressed`
    (bind _returnvalue (`LedMediaPlaybackComponent.OpenMedia` (`self.LedMediaPlayback`)))
    (if _returnvalue
      (`KismetSystemLibrary.PrintString` "Open request accepted")
      (else
        (`KismetSystemLibrary.PrintString` "Open request rejected")))))

(event `self.ReceiveBeginPlay`)

(event `Key|Nine`
  (params (Key :type "Key Structure"))
  (bind _ledmediaplayback (`self.LedMediaPlayback`))
  (:`Pressed`
    (`KismetSystemLibrary.PrintString` (`KismetStringLibrary.Conv_BoolToString` (`LedMediaPlaybackComponent.bIsOpenPending` _ledmediaplayback)))
    (`KismetSystemLibrary.PrintString` (`KismetStringLibrary.Conv_BoolToString` (`LedMediaPlaybackComponent.bIsOpened` _ledmediaplayback)))))

(event `Key|Two`
  (params (Key :type "Key Structure"))
  (:`Pressed`
    (bind _returnvalue (`LedMediaPlaybackComponent.PlayMedia` (`self.LedMediaPlayback`)))
    (if _returnvalue
      (`KismetSystemLibrary.PrintString` "Play succeeded")
      (else
        (`KismetSystemLibrary.PrintString` "Play failed")))))

(event `Key|Three`
  (params (Key :type "Key Structure"))
  (:`Pressed`
    (bind _returnvalue (`LedMediaPlaybackComponent.PauseMedia` (`self.LedMediaPlayback`)))
    (if _returnvalue
      (`KismetSystemLibrary.PrintString` "Pause succeeded")
      (else
        (`KismetSystemLibrary.PrintString` "Pause failed")))))

(event `Key|Four`
  (params (Key :type "Key Structure"))
  (:`Pressed`
    (bind _returnvalue (`LedMediaPlaybackComponent.StopMedia` (`self.LedMediaPlayback`)))
    (if _returnvalue
      (`KismetSystemLibrary.PrintString` "Stop succeeded")
      (else
        (`KismetSystemLibrary.PrintString` "Stop failed")))))

(event `Key|Five`
  (params (Key :type "Key Structure"))
  (:`Pressed`
    (bind _returnvalue (`LedMediaPlaybackComponent.SeekMedia` (`self.LedMediaPlayback`) 5.0))
    (if _returnvalue
      (`KismetSystemLibrary.PrintString` "Seek 5 sec succeeded")
      (else
        (`KismetSystemLibrary.PrintString` "Seek 5 sec failed")))))

(event `Key|Six`
  (params (Key :type "Key Structure"))
  (:`Pressed`
    (bind _returnvalue (`LedMediaPlaybackComponent.SeekMedia` (`self.LedMediaPlayback`) -1.0))
    (if _returnvalue
      (`KismetSystemLibrary.PrintString` "Seek -1.0 sec succeeded")
      (else
        (`KismetSystemLibrary.PrintString` "Seek -1.0 sec failed")))))

(event `Key|Seven`
  (params (Key :type "Key Structure"))
  (:`Pressed`
    (bind _returnvalue (`LedMediaPlaybackComponent.SeekMedia` (`self.LedMediaPlayback`) 9999.0))
    (if _returnvalue
      (`KismetSystemLibrary.PrintString` "Seek 9999.0 sec succeeded")
      (else
        (`KismetSystemLibrary.PrintString` "Seek 9999.0 sec failed")))))

(event `Key|Eight`
  (params (Key :type "Key Structure"))
  (bind _ledmediaplayback (`self.LedMediaPlayback`))
  (:`Pressed`
    (`KismetSystemLibrary.PrintString` (`KismetStringLibrary.Conv_DoubleToString` (`LedMediaPlaybackComponent.GetDurationSeconds` _ledmediaplayback)))
    (`KismetSystemLibrary.PrintString` (`KismetStringLibrary.Conv_DoubleToString` (`LedMediaPlaybackComponent.GetCurrentMediaTimeSeconds` _ledmediaplayback)))))

(fn `UserConstructionScript`)